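; BP_Tile is an infinite-terrain tile that scatters randomized props (containers, canisters, sandbags, rocks, boxes) through PlaceActors on BeginPlay.
; Its barrier starts locked (red, colliding) and unlocks green while the player overlaps LockingVolume.
; Leaving that volume relocks it and asks InfiniteTerrainGamemode to spawn another tile, with GetAttachLocation exposing the Arrow transform as the attach point.
; The tile destroys itself when the player enters DestroyVolume.
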(event `self.ReceiveBeginPlay`
  (`self.Lock`)
  (`self.PlaceActors` "/Game/Dynamic/Terrain/Props/BP_Container.BP_Container_C" 1 3 400.0)
  (`self.PlaceActors` "/Game/Dynamic/Terrain/Props/BP_Canister.BP_Canister_C" 4 9 50.0)
  (`self.PlaceActors` "/Game/Dynamic/Terrain/Props/BP_SandBags.BP_SandBags_C" 3 7 250.0 1.0 3.0)
  (`self.PlaceActors` "/Game/Dynamic/Terrain/Props/BP_Rock01.BP_Rock01_C" 0 2 150.0 1.0 5.0)
  (`self.PlaceActors` "/Game/Dynamic/Terrain/Props/BP_Rock17.BP_Rock17_C" 1 2 250.0 1.0 3.0)
  (`self.PlaceActors` "/Game/Dynamic/Terrain/Props/BP_Box.BP_Box_C" 1 1 100.0)
  (`self.PlaceActors` "/Game/Dynamic/Terrain/Props/BP_Rock05.BP_Rock05_C" 1 1 250.0))

(event `self.LockingVolume.OnComponentBeginOverlap`
  (params (OverlappedComponent :type "PrimitiveComponent Object Reference") (OtherActor :type "Actor Object Reference") (OtherComp :type "PrimitiveComponent Object Reference") (OtherBodyIndex :type Integer) (bFromSweep :type Boolean) (SweepResult :type "HitResult Structure (by ref)"))
  (`self.IsPlayerActor` OtherActor)
  (`self.Unlock`))

(event `self.LockingVolume.OnComponentEndOverlap`
  (params (OverlappedComponent :type "PrimitiveComponent Object Reference") (OtherActor :type "Actor Object Reference") (OtherComp :type "PrimitiveComponent Object Reference") (OtherBodyIndex :type Integer))
  (`self.IsPlayerActor` OtherActor)
  (`self.Lock`)
  (bind _asinfinite_terrain_gamemode (cast `/Game/Dynamic/InfiniteTerrainGamemode` (`GameplayStatics.GetGameMode`)))
  (`/Game/Dynamic/InfiniteTerrainGamemode.SpawnTile` _asinfinite_terrain_gamemode))

(event `self.DestroyVolume.OnComponentBeginOverlap`
  (params (OverlappedComponent :type "PrimitiveComponent Object Reference") (OtherActor :type "Actor Object Reference") (OtherComp :type "PrimitiveComponent Object Reference") (OtherBodyIndex :type Integer) (bFromSweep :type Boolean) (SweepResult :type "HitResult Structure (by ref)"))
  (`self.IsPlayerActor` OtherActor)
  (`self.K2_DestroyActor`))

(fn `GetAttachLocation`
  (returns (`Attach Transform` :type "Transform Structure"))
  (return (`SceneComponent.K2_GetComponentToWorld` (`self.Arrow`))))

(fn `Lock`
  (`PrimitiveComponent.SetCollisionEnabled` (`self.Barrier`) "QueryAndPhysics")
  (`PrimitiveComponent.SetMaterial` (`self.Barrier`) 0 "/Game/Dynamic/Terrain/MI_Barrier_Red.MI_Barrier_Red"))

(fn `Unlock`
  (`PrimitiveComponent.SetCollisionEnabled` (`self.Barrier`) "NoCollision")
  (`PrimitiveComponent.SetMaterial` (`self.Barrier`) 0 "/Game/Dynamic/Terrain/MI_Barrier_Green.MI_Barrier_Green"))

(fn `UserConstructionScript`)